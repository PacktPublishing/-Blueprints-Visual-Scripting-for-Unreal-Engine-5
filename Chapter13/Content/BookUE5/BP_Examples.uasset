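; BP_Examples is a collection of unrelated Blueprint scripting examples, apparently for a UE5 book.
; The event graph demonstrates flow control: Switch, DoOnce with a recharge timer, DoN with reload, FlipFlop, Gate-driven overlap damage, Sequence, MultiGate mesh cycling and ForEach.
; Functions look up prices in a map and weapons in a data table.
; Weapon firing functions are empty stubs, and many container and data table nodes are left unwired.
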(event Custom|End%20of%20Round
  (params (Winner%20name :type String))
  (Utilities|Set|Add (Variables|Default|GetUniqueNames) Winner%20name))

(event Custom|Race%20Result
  (params (Position :type Integer))
  (switch int Position
    (:1
      (Variables|Default|SetMedal%20Name "GOLD"))
    (:2
      (Variables|Default|SetMedal%20Name "SILVER"))
    (:3
      (Variables|Default|SetMedal%20Name "BRONZE"))))

(event Custom|Fire%20dual%20wield%20pistols
  (Utilities|FlowControl|FlipFlop
    (:A
      (Utilities|FireLeftPistol))
    (:B
      (Utilities|FireRightPistol))))

(event Custom|Sequence%20test
  (Utilities|FlowControl|Sequence
    (:then_0
      (Development|PrintString "FIRST")
      (if true
        (Development|PrintString "SECOND")))
    (:then_1
      (Development|PrintString "THIRD"))))

(event Custom|Turn%20on%20all%20lamps
  (for _array_element (Variables|Default|GetRoom%20Lamps)
    (Rendering|SetVisibility (Variables|/Script/Engine.PointLight|GetPointLightComponent _array_element) true false)))

(event Custom|Full%20charge
  (Utilities|FlowControl|DoOnce false ; enters at Reset
    (:Completed
      (Utilities|UseChargedWeapon
        (:Out
          (Utilities|Time|SetTimerbyEvent (delegate Custom|Full%20charge) 3e+01))))))

(event EventTick
  (params (DeltaSeconds :type Float%20%28single-precision%29))
  (Utilities|FlowControl|Gate true
    (:Exit
      (Game|Damage|ApplyDamage (stale Collision|EventActorBeginOverlap OtherActor) DeltaSeconds 0 0))))

(event Collision|EventActorBeginOverlap
  (params (OtherActor :type Actor%20Object%20Reference))
  (Utilities|FlowControl|Gate true) ; enters at Open
)

(event Collision|EventActorEndOverlap
  (params (OtherActor :type Actor%20Object%20Reference))
  (Utilities|FlowControl|Gate true) ; enters at Close
)

(event Input|KeyboardEvents|SpaceBar
  (params (Key :type Key%20Structure :default "None"))
  (:Pressed
    (Utilities|FlowControl|DoN 3
      (:Exit
        (Utilities|FireSpecialWeapon)))))

(event Input|KeyboardEvents|R
  (params (Key :type Key%20Structure :default "None"))
  (:Pressed
    (Utilities|FlowControl|DoN 3) ; enters at Reset
  ))

(event Input|KeyboardEvents|Tab
  (params (Key :type Key%20Structure :default "None"))
  (bind _decor_object (Variables|Default|GetDecor%20Object))
  (:Pressed
    (Utilities|FlowControl|MultiGate false true -1
      (:Out%200
        (Components|StaticMesh|SetStaticMesh _decor_object "/Engine/VREditor/BasicMeshes/SM_Ball_01.SM_Ball_01"))
      (:Out%201
        (Components|StaticMesh|SetStaticMesh _decor_object "/Game/StarterContent/Props/SM_Statue.SM_Statue"))
      (:Out%202
        (Components|StaticMesh|SetStaticMesh _decor_object "/Game/StarterContent/Props/SM_Bush.SM_Bush")))))

(fn ConstructionScript)

(fn CalculateTotalPrice
  (params (Product%20Name :type String) (Amount :type Float%20%28single-precision%29))
  (return (* Amount (.Value (Utilities|Map|Find (Variables|Default|GetPriceTable) Product%20Name)))))

(fn SelectWeapon
  (params (Weapon%20ID :type Name))
  (bind _returnvalue (Utilities|GetDataTableRow (Variables|Default|GetWeaponTable) Weapon%20ID)
    (:then
      (bind _output_get (Variables|Default|SetCurrentWeapon _returnvalue)) ; This is a WeaponType struct
      (Development|PrintString (.Name (Utilities|Struct|BreakWeaponType _output_get))))))