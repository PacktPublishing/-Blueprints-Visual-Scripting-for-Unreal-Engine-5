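; BP_ProceduralMeshes is an actor that procedurally lays out copies of a chosen static mesh in a flat grid.
; Its Construction Script assigns the mesh variable to an Instanced Static Mesh component, then uses nested loops to add an instance per row and column.
; Variables control the row count, instances per row and the spacing along X and Y.
; The Event Graph holds no active logic.
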(event EventBeginPlay)

(event Collision|EventActorBeginOverlap
  (params (OtherActor :type Actor%20Object%20Reference)))

(event EventTick
  (params (DeltaSeconds :type Float%20%28single-precision%29)))

(fn ConstructionScript
  (Components|StaticMesh|SetStaticMesh (Variables|Default|GetInstancedStaticMesh) (Variables|Default|GetStaticMeshVar))
  (for _index (range 1 (Variables|Default|GetNumberOfRows))
    (LocalVariables|SetInstanceLocationX (* _index (Variables|Default|GetSpaceBetweenRows)))
    (for _index_2 (range 1 (Variables|Default|GetInstancesPerRow))
      (Components|InstancedStaticMesh|AddInstance (Variables|Default|GetInstancedStaticMesh) (Math|Transform|MakeTransform (Math|Vector|MakeVector (LocalVariables|GetInstanceLocationX) (* _index_2 (Variables|Default|GetSpaceBetweenInstances)) 0.0) "0, 0, 0" "1.000000,1.000000,1.000000") false))))