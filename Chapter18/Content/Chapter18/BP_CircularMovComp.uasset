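; BP_CircularMovComp is a movement component that circles around its parent's origin at a rate set by RotationPerSecond.
; Each Tick it scales that rate by delta time, rotates its relative location around the Z axis and adds the same angle as local yaw, so its facing follows the orbit.
; Several disconnected location and rotation nodes remain in the graph and never run.
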(event EventTick
  (params (DeltaSeconds :type Float%20%28single-precision%29))
  (bind _output_get (Variables|Default|SetDeltaAngle (* DeltaSeconds (Variables|Default|GetRotationPerSecond))))
  (Transformation|SetRelativeLocation (Math|Vector|RotateVectorAroundAxis (Variables|Default|GetRelativeLocation) _output_get "0, 0,1.000000") false false)
  (Transformation|AddLocalRotation (Math|Rotator|MakeRotator 0.0 0.0 (Variables|Default|GetDeltaAngle)) false false))