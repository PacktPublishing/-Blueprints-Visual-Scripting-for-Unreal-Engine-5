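; BP_ExpLevelComp is an experience and leveling Blueprint that tracks current XP and level.
; IncreaseExperience adds points, then uses the CanLevelUp and XpReachesNewLevel macros to check for a next level in the ExpLevel threshold array and whether XP reaches it.
; It raises at most one level per call and returns the level with a LevelUp flag, which is never cleared here.
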(event EventBeginPlay)

(event EventTick
  (params (DeltaSeconds :type Float%20%28single-precision%29)))

(fn IncreaseExperience
  (params (ExperiencePoints :type Integer))
  (Variables|Default|SetCurrentXP (+ ExperiencePoints (Variables|Default|GetCurrentXP)))
  (Utilities|CanLevelUp
    (:Yes
      (Utilities|XpReachesNewLevel
        (:Yes
          (Math|Integer|IncrementInt (Variables|Default|GetCurrentLevel)
            (:%20%20
              (LocalVariables|SetLevelUpVar true))))
        (:No
          _)))
    (:No
      _))
  (return (LocalVariables|GetLevelUpVar) (Variables|Default|GetCurrentLevel)))